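; Game instance Blueprint for the menu that handles hosting, finding and joining LAN multiplayer sessions.
; Hosting creates a four-connection LAN session and, on success, opens the level as a listen server.
; Searching stores the results and tells the calling widget to show the list or reset its join state if none are found.
; Joining records the chosen session as current and joins it.
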(event Custom|Event_JoinSession
  (params (PlayerController :type Player%20Controller%20Object%20Reference) (SessionToJoin :type Blueprint%20Session%20Result%20Structure%20%28by%20ref%29))
  (Variables|Default|SetCurrentSession SessionToJoin)
  (|JoinSession PlayerController SessionToJoin))

(event Custom|Event_CreateSession
  (params (PlayerController :type Player%20Controller%20Object%20Reference))
  (|Session PlayerController 4 true
    (:OnSuccess
      (Game|OpenLevel(byObjectReference) (Variables|Default|GetLevel) true "listen"))))

(event Custom|Event_FindSession
  (params (PlayerController :type Player%20Controller%20Object%20Reference) (Widget :type WG%20Menu%20Object%20Reference))
  (bind _results (|FindSessions PlayerController -1 true)
    (:OnSuccess
      (bind _output_get (Variables|Default|SetSessionsResults _results))
      (if (Utilities|Array|IsNotEmpty _output_get)
        (Default|EventShowList Widget)
        (else
          (Default|EventResetJoin Widget))))))