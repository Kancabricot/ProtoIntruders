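; BP_ObjectToTake is a pickup actor that the player takes by interacting with it.
; The construction script sets the Object mesh from the ObjectToTake enum, using a cone for Outil and no mesh otherwise.
; On Interact it casts player character 0 to BP_ThirdPersonCharacter and passes itself to that character's RunOnServerDestroyObject to remove the object through the server.
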(event EventInteract
  (bind _asbp_third_person_character (Utilities|Casting|CastToBP_ThirdPersonCharacter (Game|GetPlayerCharacter 0)))
  (Default|RunonServerDestroyObject _asbp_third_person_character self))

(fn ConstructionScript
  (switch Utilities|FlowControl|Switch|SwitchonEnum_ObjectToTake (Variables|Default|GetObjectToTake)
    (:NewEnumerator0
      (Variables|Default|SetStaticMeshObject 0))
    (:NewEnumerator1
      (Variables|Default|SetStaticMeshObject "/Engine/BasicShapes/Cone.Cone")))
  (Components|StaticMesh|SetStaticMesh (Variables|Default|GetObject) (Variables|Default|GetStaticMeshObject)))