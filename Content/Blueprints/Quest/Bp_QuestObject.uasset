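; Bp_QuestObject is an interactable quest item that completes the interacting player's current quest when its type matches.
; On Interact, it compares WhatsObject with the player's ActuQuest for the two handled quest IDs and sets HasCompleteIsQuest on a match.
; It then has itself destroyed through the player's RunOnServerDestroyObject call.
; The construction script picks a cone or sphere mesh from WhatsObject.
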(event EventBeginPlay)

(event Collision|EventActorBeginOverlap
  (params (OtherActor :type Actor%20Object%20Reference)))

(event EventTick
  (params (DeltaSeconds :type Float%20%28single-precision%29)))

(event EventInteract
  (params (Player :type BP%20Third%20Person%20Character%20Object%20Reference))
  (Variables|Default|SetPlayer Player)
  (switch int (Variables|/Game/ThirdPerson/Blueprints/BP_ThirdPersonCharacter.BP_ThirdPersonCharacter_C|GetActuQuest Player)
    (:0
      (if (== (Variables|Default|GetWhatsObject) (Variables|/Game/ThirdPerson/Blueprints/BP_ThirdPersonCharacter.BP_ThirdPersonCharacter_C|GetActuQuest (Variables|Default|GetPlayer)))
        (Variables|/Game/ThirdPerson/Blueprints/BP_ThirdPersonCharacter.BP_ThirdPersonCharacter_C|SetHasCompleteIsQuest (Variables|Default|GetPlayer) true)
        (Default|RunonServerDestroyObject (Variables|Default|GetPlayer) self :!label _label)))
    (:1
      (if (== (Variables|Default|GetWhatsObject) (Variables|/Game/ThirdPerson/Blueprints/BP_ThirdPersonCharacter.BP_ThirdPersonCharacter_C|GetActuQuest (Variables|Default|GetPlayer)))
        (Variables|/Game/ThirdPerson/Blueprints/BP_ThirdPersonCharacter.BP_ThirdPersonCharacter_C|SetHasCompleteIsQuest (Variables|Default|GetPlayer) true)
        (goto _label)))))

(fn ConstructionScript
  (switch int (Variables|Default|GetWhatsObject)
    (:0
      (Components|StaticMesh|SetStaticMesh (Variables|Default|GetSphere) "/Engine/BasicShapes/Cone.Cone"))
    (:1
      (Components|StaticMesh|SetStaticMesh (Variables|Default|GetSphere) "/Engine/BasicShapes/Sphere.Sphere"))))