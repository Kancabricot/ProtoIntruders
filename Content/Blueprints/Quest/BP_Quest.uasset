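; BP_Quest assigns a quest to a player and shows its French objective text on that player's quest HUD.
; ChooseQuest runs through a DoOnce, so only the first call stores the player and quest index, then switches on the index.
; Each case pulls hardcoded text from a Quest function (retrieve objects, damage or repair a generator) and prints debug output.
; Quest5 is an unused empty stub, and completion is not tracked here.
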(event Custom|ChooseQuest
  (params (Quest :type Integer) (Player :type BP%20Third%20Person%20Character%20Object%20Reference))
  (Utilities|FlowControl|DoOnce false
    (:Completed
      (Variables|Default|SetActuPlayer Player)
      (bind _output_get (Variables|Default|SetActuQuest Quest))
      (Development|PrintString "dsqf")
      (switch int _output_get
        (:0
          (bind _newparam (CallFunction|Quest1))
          (Default|SetText (Variables|/Game/ThirdPerson/Blueprints/BP_ThirdPersonCharacter.BP_ThirdPersonCharacter_C|GetQuestHud (Variables|Default|GetActuPlayer)) _newparam)
          (Development|PrintString "0"))
        (:1
          (bind _newparam_2 (CallFunction|Quest2))
          (Default|SetText (Variables|/Game/ThirdPerson/Blueprints/BP_ThirdPersonCharacter.BP_ThirdPersonCharacter_C|GetQuestHud (Variables|Default|GetActuPlayer)) _newparam_2)
          (Development|PrintString "1"))
        (:2
          (bind _newparam_3 (CallFunction|Quest3))
          (Default|SetText (Variables|/Game/ThirdPerson/Blueprints/BP_ThirdPersonCharacter.BP_ThirdPersonCharacter_C|GetQuestHud (Variables|Default|GetActuPlayer)) _newparam_3)
          (Development|PrintString "2"))
        (:3
          (bind _newparam_4 (CallFunction|Quest4))
          (Default|SetText (Variables|/Game/ThirdPerson/Blueprints/BP_ThirdPersonCharacter.BP_ThirdPersonCharacter_C|GetQuestHud (Variables|Default|GetActuPlayer)) _newparam_4)
          (Development|PrintString "3"))))))

(fn ConstructionScript)

(fn Quest1
  (return "Récupérer l’objet A"))

(fn Quest2
  (return "Récupérer l’objet B"))

(fn Quest3
  (return "Endommager le générateur électrique 1 fois"))

(fn Quest4
  (return "éparer le générateur électrique 1 fois"))

(fn Quest5
  (return ""))