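; BP_Generateur is a generator that switches the level's lighting between broken and repaired states.
; GenerateurEvent reads the IsBreak flag and calls RepearLight or DestroyLight to toggle the state.
; Each handler finds every Light actor with GetAllActorsOfClass, sets its intensity to zero or one fixed value, and updates IsBreak.
; Repair applies that same intensity to all lights rather than restoring their original values.
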(event Custom|DestroyLight
  (bind _outactors (Actor|GetAllActorsOfClass "/Script/Engine.Light"))
  (for _array_element _outactors
    (Rendering|Components|Light|SetIntensity (Variables|/Script/Engine.Light|GetLightComponent _array_element) 0.0)
    (Variables|Default|SetIsBreak true)))

(event Custom|RepearLight
  (bind _outactors (Actor|GetAllActorsOfClass "/Script/Engine.Light"))
  (for _array_element _outactors
    (Rendering|Components|Light|SetIntensity (Variables|/Script/Engine.Light|GetLightComponent _array_element) 44.788933)
    (Variables|Default|SetIsBreak false)))

(event Custom|GenerateurEvent
  (if (Variables|Default|GetIsBreak)
    (CallFunction|RepearLight)
    (else
      (CallFunction|DestroyLight))))

(event EventBeginPlay)

(event Collision|EventActorBeginOverlap
  (params (OtherActor :type Actor%20Object%20Reference)))

(event EventTick
  (params (DeltaSeconds :type Float%20%28single-precision%29)))

(fn ConstructionScript)