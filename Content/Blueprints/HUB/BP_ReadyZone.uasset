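; BP_ReadyZone is a hub trigger zone that sends the session to ThirdPersonMap when a player character is inside it.
; Sphere overlap begin and end pass +1 or -1 to a ready-player event, apparently meant to run on the server, which updates and prints the count.
; Whenever the count is at least one, it runs a ServerTravel console command once per character, using the loop index to pick each player controller.
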(event OnComponentBeginOverlap(Sphere)
  (params (OverlappedComponent :type Primitive%20Component%20Object%20Reference) (OtherActor :type Actor%20Object%20Reference) (OtherComp :type Primitive%20Component%20Object%20Reference) (OtherBodyIndex :type Integer) (bFromSweep :type Boolean) (SweepResult :type Hit%20Result%20Structure%20%28by%20ref%29))
  (Utilities|Casting|CastToBP_ThirdPersonCharacter OtherActor)
  (CallFunction|RunonServeurPLayerReady 1))

(event OnComponentEndOverlap(Sphere)
  (params (OverlappedComponent :type Primitive%20Component%20Object%20Reference) (OtherActor :type Actor%20Object%20Reference) (OtherComp :type Primitive%20Component%20Object%20Reference) (OtherBodyIndex :type Integer))
  (Utilities|Casting|CastToBP_ThirdPersonCharacter OtherActor)
  (CallFunction|RunonServeurPLayerReady -1))

(event Custom|RunOnServeur_PLayerReady
  (params (+/- :type Integer))
  (bind _output_get (Variables|Default|SetNumberOfPlayerReady (+ (Variables|Default|GetNumberOfPlayerReady) +/-)))
  (Development|PrintString (Utilities|String|ToString(Integer) _output_get))
  (if (not (< _output_get 1))
    (bind _outactors (Actor|GetAllActorsOfClass "/Game/ThirdPerson/Blueprints/BP_ThirdPersonCharacter.BP_ThirdPersonCharacter_C"))
    (for (_ _array_index) _outactors
      (Development|ExecuteConsoleCommand "ServerTravel ThirdPersonMap" (Game|GetPlayerController _array_index)))))

(fn ConstructionScript)