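; Interactable door that routes open and close requests through the player character's RunOnServerOpenCloseDoor, cached at BeginPlay from player index 0.
; Interact checks that character's open flag: if false, it shows a single WG_OpenDoor widget; if true, it toggles the door directly.
; OpenCloseDoorCall clears the widget reference, sends the request and blocks interaction for a short cooldown.
; Reset clears the widget reference so the prompt can be created again.
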(event Custom|OpenCloseDoorCall
  (Variables|Default|SetWidgetRef 0)
  (Variables|Default|Setb_CanOpen false)
  (Default|RunonServerOpenCloseDoor (Variables|Default|GetPlayerRef) (Variables|Default|GetDoor))
  (Utilities|FlowControl|Delay 1.5)
  (Variables|Default|Setb_CanOpen true))

(event Custom|Reset
  (Variables|Default|SetWidgetRef 0))

(event EventBeginPlay
  (bind _asbp_third_person_character (Utilities|Casting|CastToBP_ThirdPersonCharacter (Game|GetPlayerCharacter 0)))
  (Variables|Default|SetPlayerRef _asbp_third_person_character))

(event EventInteract
  (params (Player :type BP%20Third%20Person%20Character%20Object%20Reference))
  (if (Variables|Default|Getb_CanOpen)
    (if (not (Variables|/Game/ThirdPerson/Blueprints/BP_ThirdPersonCharacter.BP_ThirdPersonCharacter_C|Getb_IsOpen (Variables|Default|GetPlayerRef)))
      (if (== (Variables|Default|GetWidgetRef) 0)
        (bind _returnvalue (UserInterface|CreateWidget "/Game/Widget/Door/WG_OpenDoor.WG_OpenDoor_C"))
        (bind _output_get (Variables|Default|SetWidgetRef _returnvalue))
        (Default|GetRef _output_get self Player)
        (UserInterface|Viewport|AddtoViewport _output_get 0))
      (else
        (CallFunction|OpenCloseDoorCall)))))

(fn ConstructionScript)