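; Timer actor that counts minutes and seconds of play and opens the ships once a set minute is reached.
; Tick uses a one-second Delay to advance the clock, shows the WG_ShipOpen widget once a minute before ShipTime, then sets IsOpen on every BP_Ship during that minute.
; BeginPlay's random ShipTime range is fixed at 2, WhatShip is rolled but unused, and the Srv/Client events are unused stubs.
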(event Custom|Srv
  (CallFunction|Client))

(event Custom|Client)

(event EventBeginPlay
  (Variables|Default|SetShipTime (Math|Random|RandomIntegerinRange 2 2))
  (Variables|Default|SetWhatShip (Math|Random|RandomIntegerinRange 1 3)))

(event Collision|EventActorBeginOverlap
  (params (OtherActor :type Actor%20Object%20Reference)))

(event EventTick
  (params (DeltaSeconds :type Float%20%28single-precision%29))
  (Utilities|FlowControl|Sequence
    (:then_0
      (Utilities|FlowControl|Delay 1.0)
      (Variables|Default|SetSeconde (+ (Variables|Default|GetSeconde) 1))
      (if (> (Variables|Default|GetSeconde) 59)
        (Variables|Default|SetMinutes (+ (Variables|Default|GetMinutes) 1))
        (Variables|Default|SetSeconde 0)))
    (:then_1
      (if (== (Variables|Default|GetMinutes) (Variables|Default|GetShipTime))
        (bind _outactors (Actor|GetAllActorsOfClass "/Game/Blueprints/Evacuqtion/Ship/BP_Ship.BP_Ship_C"))
        (for _array_element _outactors
          (Variables|/Game/Blueprints/Evacuqtion/Ship/BP_Ship.BP_Ship_C|SetIsOpen _array_element true))
        (elif (== (Variables|Default|GetMinutes) (- (Variables|Default|GetShipTime) 1))
          (Utilities|FlowControl|DoOnce false
            (:Completed
              (bind _returnvalue (UserInterface|CreateWidget "/Game/Blueprints/Evacuqtion/Ship/WG_ShipOpen.WG_ShipOpen_C"))
              (UserInterface|Viewport|AddtoViewport _returnvalue 0))))))))

(fn ConstructionScript)