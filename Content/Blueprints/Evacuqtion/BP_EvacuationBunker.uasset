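; Evacuation bunker that removes players who have completed their quest when they overlap its box, switching them to spectating and destroying their character.
; It starts open, hiding component R by teleporting it to a far-off position, and closing returns R to its saved location.
; Open and close pass through Serv-to-Client event pairs, though nothing here calls close.
; A generator-based open check is left unconnected.
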(event OnComponentBeginOverlap(Box)
  (params (OverlappedComponent :type Primitive%20Component%20Object%20Reference) (OtherActor :type Actor%20Object%20Reference) (OtherComp :type Primitive%20Component%20Object%20Reference) (OtherBodyIndex :type Integer) (bFromSweep :type Boolean) (SweepResult :type Hit%20Result%20Structure%20%28by%20ref%29))
  (bind _asbp_third_person_character (Utilities|Casting|CastToBP_ThirdPersonCharacter OtherActor))
  (bind _output_get (Variables|Default|SetPlayerRef _asbp_third_person_character))
  (if (Variables|/Game/ThirdPerson/Blueprints/BP_ThirdPersonCharacter.BP_ThirdPersonCharacter_C|GetHasCompleteIsQuest _output_get)
    (Default|Spectatesrv (Variables|Default|GetPlayerRef))
    (Actor|DestroyActor (Variables|Default|GetPlayerRef))))

(event Custom|openServ
  (CallFunction|OpenClient))

(event Custom|OpenClient
  (Variables|Default|SetIsOpen true)
  (Transformation|SetWorldLocation (Variables|Default|Getr) "10000.000000,10000.000000,10000.000000" false false))

(event Custom|CloseServ
  (CallFunction|CloseClient))

(event Custom|CloseClient
  (Variables|Default|SetIsOpen false)
  (Transformation|SetWorldLocation (Variables|Default|Getr) (Variables|Default|GetDefaultPos) false false))

(event EventBeginPlay
  (Variables|Default|SetDefaultPos (Transformation|GetWorldLocation (Variables|Default|Getr)))
  (CallFunction|OpenServ))

(fn ConstructionScript)