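; BP_Ship is an evacuation ship that reacts when a third-person character enters its box trigger while it is open.
; On BeginPlay it caches the level's Bp_Timer, whose WhatShip value is compared with the ship's own ShipType on overlap.
; A match calls Spectatesrv on the character, while a mismatch sets the character's movement-disable flag for a few seconds as a penalty.
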(event OnComponentBeginOverlap(Box)
  (params (OverlappedComponent :type Primitive%20Component%20Object%20Reference) (OtherActor :type Actor%20Object%20Reference) (OtherComp :type Primitive%20Component%20Object%20Reference) (OtherBodyIndex :type Integer) (bFromSweep :type Boolean) (SweepResult :type Hit%20Result%20Structure%20%28by%20ref%29))
  (bind _asbp_third_person_character (Utilities|Casting|CastToBP_ThirdPersonCharacter OtherActor))
  (if (Variables|Default|GetIsOpen)
    (if (== (Variables|Default|GetShipType) (Variables|/Game/Blueprints/Timer/bp_Timer.bp_Timer_C|GetWhatShip (Variables|Default|GetTimerRef)))
      (Default|Spectatesrv _asbp_third_person_character)
      (else
        (Variables|/Game/ThirdPerson/Blueprints/BP_ThirdPersonCharacter.BP_ThirdPersonCharacter_C|SetDiseableMouvement _asbp_third_person_character true)
        (Utilities|FlowControl|Delay 3.0)
        (Variables|/Game/ThirdPerson/Blueprints/BP_ThirdPersonCharacter.BP_ThirdPersonCharacter_C|SetDiseableMouvement _asbp_third_person_character false)))))

(event EventBeginPlay
  (bind _returnvalue (Actor|GetActorOfClass "/Game/Blueprints/Timer/bp_Timer.bp_Timer_C"))
  (Variables|Default|SetTimerRef _returnvalue))

(event Collision|EventActorBeginOverlap
  (params (OtherActor :type Actor%20Object%20Reference)))

(event EventTick
  (params (DeltaSeconds :type Float%20%28single-precision%29)))

(fn ConstructionScript)